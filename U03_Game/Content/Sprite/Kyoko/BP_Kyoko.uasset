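; BP_Kyoko is a Paper2D flipbook character, Kyoko, that plays animations in response to spawning and taking damage.
; On BeginPlay it plays "Start", and on AnyDamage it plays "Dab", each returning to "Idle" afterwards.
; SetFlipbook looks up the named flipbook in a map, applies it and returns its total duration, which times a Retriggerable Delay before the switch to idle.
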(event EventBeginPlay
  (bind _returnvalue (CallFunction|SetFlipbook "Start"))
  (Utilities|FlowControl|RetriggerableDelay _returnvalue)
  (CallFunction|SetFlipbook "Idle"))

(event Game|Damage|EventAnyDamage
  (params (Damage :type Float%20%28single-precision%29) (DamageType :type Damage%20Type%20Object%20Reference) (InstigatedBy :type Controller%20Object%20Reference) (DamageCauser :type Actor%20Object%20Reference))
  (bind _returnvalue (CallFunction|SetFlipbook "Dab"))
  (Utilities|FlowControl|RetriggerableDelay _returnvalue)
  (CallFunction|SetFlipbook "Idle"))

(fn ConstructionScript)

(fn SetFlipbook
  (params (InName :type Name))
  (bind _flipbooks (Variables|Default|GetFlipbooks))
  (bind _value (Utilities|Map|Find _flipbooks InName))
  (Sprite|SetFlipbook (Variables|Default|GetPaperFlipbook) _value)
  (return (Class|PaperFlipbook|GetTotalDuration _value)))